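; Enemy AI character that chases the player and performs a melee attack on reaching them.
; PawnSensing sightings set IsSeeingPawn and call FollowPlayer, which uses AIMoveTo toward the player character and plays a backhand montage on success.
; CanAttack gates the attack for the montage's duration but is re-armed on every FollowPlayer call.
; Tick halts movement until the first sighting, as IsSeeingPawn effectively never clears afterward.
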(event OnSeePawn(PawnSensing)
  (params (Pawn :type Pawn%20Object%20Reference))
  (Variables|Default|SetIsSeeingPawn true)
  (CallFunction|FollowPlayer))

(event Custom|FollowPlayer
  (Variables|Default|SetcanAttack? true)
  (if (Variables|Default|GetIsSeeingPawn)
    (AI|AIMoveTo self "0, 0, 0" (Game|GetPlayerCharacter 0) 3.0 false
      (:OnSuccess
        (if (Variables|Default|GetcanAttack?)
          (Variables|Default|SetcanAttack? false)
          (bind _returnvalue (Animation|PlayAnimMontage "/Game/AI/AI_BluePrints/StandingMeleeAttackBackhand_UE_Montage.StandingMeleeAttackBackhand_UE_Montage" 1.0 "None"))
          (Utilities|FlowControl|Delay _returnvalue)
          (Variables|Default|SetcanAttack? true))))
    (else
      (Variables|Default|SetIsSeeingPawn false))))

(event EventBeginPlay)

(event Collision|EventActorBeginOverlap
  (params (OtherActor :type Actor%20Object%20Reference)))

(event EventTick
  (params (DeltaSeconds :type Float%20%28single-precision%29))
  (if (not (Variables|Default|GetIsSeeingPawn))
    (Components|Movement|StopMovementImmediately (Variables|Character|GetCharacterMovement))))

(fn ConstructionScript)