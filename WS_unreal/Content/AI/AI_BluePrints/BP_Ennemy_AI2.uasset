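; Enemy AI pawn Blueprint that chases the player and attacks on reaching them.
; When PawnSensing sees a pawn, it sets a seeing flag and calls FollowPlayer, which moves it toward the player character with AIMoveTo.
; On a successful move, if CanAttack is set it clears that flag and calls PlayAnimMontage.
; Neither flag is reset in this graph.
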(event OnSeePawn(PawnSensing)
  (params (Pawn :type Pawn%20Object%20Reference))
  (Variables|Default|SetIsSeeingPawn true)
  (CallFunction|FollowPlayer))

(event Custom|FollowPlayer
  (if (Variables|Default|GetIsSeeingPawn)
    (AI|AIMoveTo self "0, 0, 0" (Game|GetPlayerCharacter 0) 7e+01 false
      (:OnSuccess
        (if (Variables|Default|GetcanAttack?)
          (Variables|Default|SetcanAttack? false)
          (Animation|PlayAnimMontage 0 1.0 "None"))))))

(fn ConstructionScript)