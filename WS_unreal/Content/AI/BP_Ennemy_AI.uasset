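; Enemy AI character that chases player 0 once PawnSensing spots a pawn.
; The sighting sets IsSeeingPlayer, which is never cleared, and issues an AI MoveTo toward the player.
; On Tick, while the flag is set and movement speed is not above a low threshold, a macro applies a velocity-change impulse to Box and fires RadialForce, followed by a debug print.
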(event OnSeePawn(PawnSensing)
  (params (Pawn :type Pawn%20Object%20Reference))
  (Variables|Default|SetisSeeingPlayer true)
  (CallFunction|FollowPlayer))

(event Custom|FollowPlayer
  (if (Variables|Default|GetisSeeingPlayer)
    (AI|AIMoveTo self "0, 0, 0" (Game|GetPlayerCharacter 0) 5.0 false)))

(event Collision|EventActorBeginOverlap
  (params (OtherActor :type Actor%20Object%20Reference)))

(event EventTick
  (params (DeltaSeconds :type Float%20%28single-precision%29))
  (if (not (Class|MovementComponent|IsExceedingMaxSpeed (Variables|Character|GetCharacterMovement) 1e+01))
    (if (Variables|Default|GetisSeeingPlayer)
      (Utilities|NewMacro)
      (Development|PrintString "Hello" true true "(R=1.000000,G=0.092738,B=0.000000,A=1.000000)"))))

(fn ConstructionScript)